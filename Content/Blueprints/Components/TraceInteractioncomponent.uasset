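; A scene component for trace-based interaction that forwards activate down and up presses to a focused object as messages, with the current hit and instigator.
; A helper sphere-traces forward from the component on the Visibility channel, and another stores a hit's actor and component.
; Enable and Disable toggle a gate on Tick, but nothing follows it, and no graph here calls the helpers or updates the focus.
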(event `self.ReceiveTick`
  (params (DeltaSeconds :type "Float (single-precision)"))
  (`/Engine/EditorBlueprintResources/StandardMacros.Gate` false :!label _label))

(event `Enable`
  (goto _label :!via `Open`))

(event `Disable`
  (goto _label :!via `Close`))

(event `ActivateDown`
  (params (Instigator :type "Pawn Object Reference"))
  (message `/Game/Blueprints/Interfaces/TraceInteractionInterface.TraceActivateDown` (`self.FocusedObject`) (`self.CurrentHit`) Instigator))

(event `ActivateUp`
  (params (Instigator :type "Pawn Object Reference"))
  (message `/Game/Blueprints/Interfaces/TraceInteractionInterface.TraceActivateUp` (`self.FocusedObject`) (`self.CurrentHit`) Instigator))

(fn `InteractWithHit`
  (params (Hit :type "HitResult Structure"))
  (locals (InHit :type "HitResult Structure") (InHitActor :type "Actor Object Reference") (InHitComponent :type "PrimitiveComponent Object Reference"))
  (bind _output_get (set `local.InHit` Hit))
  (bind (_bblockinghit _binitialoverlap _time _distance _location _impactpoint _normal _impactnormal _physmat _hitactor _hitcomponent) (`GameplayStatics.BreakHitResult` _output_get))
  (set `local.InHitActor` _hitactor)
  (set `local.InHitComponent` _hitcomponent))

(fn `SphereTrace`
  (params (Distance :type "Float (double-precision)") (Radius :type "Float (double-precision)"))
  (returns (Hit :type "HitResult Structure"))
  (bind _returnvalue (`self.K2_GetComponentLocation`))
  (bind _outhit (`KismetSystemLibrary.SphereTraceSingle` _returnvalue (+ _returnvalue (* (`self.GetForwardVector`) Distance)) Radius "TraceTypeQuery1"))
  (return _outhit))